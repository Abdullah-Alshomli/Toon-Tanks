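; BP_MyToonTanksGameMode is the game mode for Toon Tanks, handling the start and end-of-game screens.
; StartGame creates the start-game widget and adds it to the viewport.
; GameOver creates an end-game widget and sets its display text to a win or loss message based on the WonGame flag.
; BeginPlay and Tick are disabled stubs.
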(event EventBeginPlay)

(event EventTick
  (params (DeltaSeconds :type Float%20%28single-precision%29)))

(event EventStartGame
  (bind _returnvalue (UserInterface|CreateWidget "/Game/Blueprints/WIdgets/WBP_StartGameWidget.WBP_StartGameWidget_C"))
  (UserInterface|Viewport|AddtoViewport _returnvalue 0))

(event EventGameOver
  (params (bWonGame :type Boolean))
  (bind _returnvalue (UserInterface|CreateWidget "/Game/Blueprints/WIdgets/WBP_EndGameWidget.WBP_EndGameWidget_C"))
  (UserInterface|Viewport|AddtoViewport _returnvalue 0)
  (if bWonGame
    (Variables|Default|SetGameOverText "YOU WON!!!")
    (else
      (Variables|Default|SetGameOverText "YOU LOST!")))
  (Rendering|Components|TextRender|SetText (Variables|/Game/Blueprints/WIdgets/WBP_EndGameWidget.WBP_EndGameWidget_C|GetDisplayText _returnvalue) (Variables|Default|GetGameOverText)))

(fn ConstructionScript)